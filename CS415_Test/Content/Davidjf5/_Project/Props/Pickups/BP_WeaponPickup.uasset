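; BP_WeaponPickup is a weapon pickup actor that gives the interacting character a weapon.
; Its Interact event calls SpawnWeapon on that character, passing its configured WeaponToSpawn and its own location, then destroys itself.
; BeginPlay, overlap and Tick are disabled stubs, and the construction script only calls its parent.
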(event EventBeginPlay
  (|CallParentFunction) ; This node is disabled and will not be called.\nDrag off pins to build functionality.
)

(event Collision|EventActorBeginOverlap
  (params (OtherActor :type Actor%20Object%20Reference))
  (|CallParentFunction OtherActor) ; This node is disabled and will not be called.\nDrag off pins to build functionality.
)

(event EventTick
  (params (DeltaSeconds :type Float%20%28single-precision%29))
  (|CallParentFunction DeltaSeconds) ; This node is disabled and will not be called.\nDrag off pins to build functionality.
)

(event EventInteract
  (params (Character%20Picking%20Up :type BP%20First%20Person%20Character%20Main%20Object%20Reference))
  (Default|SpawnWeapon Character%20Picking%20Up (Variables|Default|GetWeaponToSpawn) (Transformation|GetActorLocation))
  (Actor|DestroyActor))

(fn ConstructionScript
  (|CallParentFunction))