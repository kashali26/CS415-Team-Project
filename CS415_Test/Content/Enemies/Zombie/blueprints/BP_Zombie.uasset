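; Zombie enemy that takes damage from first-person projectiles and shows its health on a widget component.
; Capsule overlap with a projectile applies damage read from its weapon class defaults, plays a sound and prints debug text.
; AnyDamage scales damage by 100, subtracts it from health and updates the WBP_EnemyHealth bar initialized on BeginPlay.
; At zero health it attaches a fire effect and destroys itself after a short delay.
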(event OnComponentBeginOverlap(CapsuleComponent)
  (params (OverlappedComponent :type Primitive%20Component%20Object%20Reference) (OtherActor :type Actor%20Object%20Reference) (OtherComp :type Primitive%20Component%20Object%20Reference) (OtherBodyIndex :type Integer) (bFromSweep :type Boolean) (SweepResult :type Hit%20Result%20Structure%20%28by%20ref%29))
  (bind _asbp_first_person_projectile_main (Utilities|Casting|CastToBP_FirstPersonProjectileMain OtherActor)
    (:then
      ;[1 1 1] Apply Damage
      (Utilities|IsValid _asbp_first_person_projectile_main
        (:Is%20Valid
          (Development|PrintString (Utilities|String|ToString(Float) (.Damage (Utilities|GetClassDefaults (Variables|/Game/Davidjf5/_Project/WeaponPickupBlueprints/Projectiles/BP_FirstPersonProjectileMain.BP_FirstPersonProjectileMain_C|GetWeapon%20Class%20 _asbp_first_person_projectile_main)))))
          (Game|Damage|ApplyDamage self (.Damage (Utilities|GetClassDefaults (Variables|/Game/Davidjf5/_Project/WeaponPickupBlueprints/Projectiles/BP_FirstPersonProjectileMain.BP_FirstPersonProjectileMain_C|GetWeapon%20Class%20 _asbp_first_person_projectile_main))) 0 0)
          (Audio|PlaySound2D 0 1.0 1.0 0.0 0 0)
          (Development|PrintString "Hit Hellhound!"))))
    (:CastFailed
      (Development|PrintString "Failed"))))

(event EventBeginPlay
  ;[1 1 1] Set Current Health
  (bind _aswbp_enemy_health (Utilities|Casting|CastToWBP_EnemyHealth (UserInterface|GetUserWidgetObject (Variables|Default|GetWidget))))
  (bind _output_get (Variables|Default|SetWBP%20Enemy%20Health _aswbp_enemy_health))
  (Variables|/Game/Enemies/EnemyHealthSystem/UI/WBP_EnemyHealth.WBP_EnemyHealth_C|SetCurrentHealth _output_get (Variables|Default|GetCurrentHealth))
  (Variables|/Game/Enemies/EnemyHealthSystem/UI/WBP_EnemyHealth.WBP_EnemyHealth_C|SetMaxHealth _output_get (Variables|Default|GetMaxHealth)))

(event Game|Damage|EventAnyDamage
  (params (Damage :type Float%20%28single-precision%29) (DamageType :type Damage%20Type%20Object%20Reference) (InstigatedBy :type Controller%20Object%20Reference) (DamageCauser :type Actor%20Object%20Reference))
  ;[1 1 1] Damage Taken
  (bind _output_get (Variables|Default|SetCurrentHealth (- (Variables|Default|GetCurrentHealth) (* Damage 1e+02))))
  (Default|UpdateHealth (Variables|Default|GetWBP%20Enemy%20Health) (Math|Integer|Clamp(Integer) _output_get 0 (Variables|Default|GetMaxHealth)))
  (if (<= (Variables|Default|GetCurrentHealth) 0)
    (Effects|SpawnEmitterAttached "/Game/StarterContent/Particles/P_Fire.P_Fire" (Variables|Collision|GetCapsuleComponent) "None")
    (Utilities|FlowControl|Delay 2.0)
    (Actor|DestroyActor)))

(fn ConstructionScript)