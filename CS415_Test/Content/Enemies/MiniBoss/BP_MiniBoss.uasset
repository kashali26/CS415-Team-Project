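; Miniboss enemy that repeatedly chases the player with AIMoveTo and deals contact damage on capsule overlap.
; Projectile overlaps apply damage from the weapon class defaults, updating health and its widget.
; At low health its acceleration is raised.
; On death it plays fire, destroys itself after a delay, adds score, and decrements the player's MinibossCount, starting the next round when miniboss, zombie and hellhound counts are depleted.
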(event OnComponentBeginOverlap(CapsuleComponent)
  (params (OverlappedComponent :type Primitive%20Component%20Object%20Reference) (OtherActor :type Actor%20Object%20Reference) (OtherComp :type Primitive%20Component%20Object%20Reference) (OtherBodyIndex :type Integer) (bFromSweep :type Boolean) (SweepResult :type Hit%20Result%20Structure%20%28by%20ref%29))
  ;[1 1 1] Damage logic
  (bind _asbp_first_person_projectile_main (Utilities|Casting|CastToBP_FirstPersonProjectileMain OtherActor)
    (:then
      (Utilities|IsValid _asbp_first_person_projectile_main
        (:Is%20Valid
          (Development|PrintString (Utilities|String|ToString(Float) (.Damage (Utilities|GetClassDefaults (Variables|/Game/Davidjf5/_Project/WeaponPickupBlueprints/Projectiles/BP_FirstPersonProjectileMain.BP_FirstPersonProjectileMain_C|GetWeapon%20Class%20 _asbp_first_person_projectile_main)))))
          (bind _returnvalue (Game|Damage|ApplyDamage self (.Damage (Utilities|GetClassDefaults (Variables|/Game/Davidjf5/_Project/WeaponPickupBlueprints/Projectiles/BP_FirstPersonProjectileMain.BP_FirstPersonProjectileMain_C|GetWeapon%20Class%20 _asbp_first_person_projectile_main))) 0 0))
          (Development|PrintString (Utilities|String|ToString(Float) _returnvalue))
          (Audio|PlaySound2D 0 1.0 1.0 0.0 0 0)
          (Development|PrintString "Hit Hellhound!"))))
    (:CastFailed
      (bind _asbp_first_person_character_main (Utilities|Casting|CastToBP_FirstPersonCharacterMain OtherActor))
      (bind _returnvalue_2 (Game|Damage|ApplyDamage _asbp_first_person_character_main 3e+01 0 0))
      (Development|PrintText (Utilities|Text|ToText(Float) _returnvalue_2 "HalfToEven") true true "(R=1.000000,G=0.000000,B=0.214302,A=1.000000)"))))

(event Custom|Chase%20Player
  (bind _asbp_first_person_character_main (Utilities|Casting|CastToBP_FirstPersonCharacterMain (Game|GetPlayerCharacter 0))
    (:then
      (AI|AIMoveTo self "0, 0, 0" _asbp_first_person_character_main 5.0 false
        (:OnSuccess
          _)
        (:OnFail
          (Development|PrintText "Failed Move To" true true "(R=0.000000,G=0.660000,B=1.000000,A=1.000000)" 1e+01)))
      (CallFunction|ChasePlayer))
    (:CastFailed
      (Development|PrintText "NOT BP PLAYER"))))

(event EventBeginPlay
  ;[1 1 1] Set Current Health
  (Utilities|FlowControl|Sequence
    (:then_0
      (bind _aswbp_enemy_health (Utilities|Casting|CastToWBP_EnemyHealth (UserInterface|GetUserWidgetObject (Variables|Default|GetWidget))))
      (bind _output_get (Variables|Default|SetWBP%20Enemy%20Health _aswbp_enemy_health))
      (Variables|/Game/Enemies/EnemyHealthSystem/UI/WBP_EnemyHealth.WBP_EnemyHealth_C|SetCurrentHealth _output_get (Variables|Default|GetCurrentHealth))
      (Variables|/Game/Enemies/EnemyHealthSystem/UI/WBP_EnemyHealth.WBP_EnemyHealth_C|SetMaxHealth _output_get (Variables|Default|GetMaxHealth))
      (CallFunction|ChasePlayer))
    (:then_1
      (Utilities|FlowControl|Delay 2.0)
      (bind _asbp_first_person_character_main (Utilities|Casting|CastToBP_FirstPersonCharacterMain (Game|GetPlayerCharacter 0)))
      (Variables|Default|SetCharacter%20Ref _asbp_first_person_character_main)
      (Variables|Default|SetUI%20Ref (Variables|/Game/Davidjf5/_Project/Assets/Character/Soldier/Blueprints/BP_FirstPersonCharacterMain.BP_FirstPersonCharacterMain_C|GetOverlapUI%20Widget _asbp_first_person_character_main)))))

(event Game|Damage|EventAnyDamage
  (params (Damage :type Float%20%28single-precision%29) (DamageType :type Damage%20Type%20Object%20Reference) (InstigatedBy :type Controller%20Object%20Reference) (DamageCauser :type Actor%20Object%20Reference))
  (bind _ui_ref (Variables|Default|GetUI%20Ref))
  (bind _character_ref (Variables|Default|GetCharacter%20Ref))
  ;[1 1 1] Damage Taken
  (bind _output_get (Variables|Default|SetCurrentHealth (- (Variables|Default|GetCurrentHealth) (* Damage 1.0))))
  (Default|UpdateHealth (Variables|Default|GetWBP%20Enemy%20Health) (Math|Integer|Clamp(Integer) _output_get 0 (Variables|Default|GetMaxHealth)))
  (if (<= (Variables|Default|GetCurrentHealth) 0)
    (Effects|SpawnEmitterAttached "/Game/StarterContent/Particles/P_Fire.P_Fire" (Variables|Collision|GetCapsuleComponent) "None")
    (Utilities|FlowControl|Delay 2.0)
    (Actor|DestroyActor)
    (Variables|/Game/HealthAndAmmoScreen/WBP_OverlapUI.WBP_OverlapUI_C|SetCurrent%20Score _ui_ref (+ 10000 (Variables|/Game/HealthAndAmmoScreen/WBP_OverlapUI.WBP_OverlapUI_C|GetCurrent%20Score _ui_ref)))
    (bind _result (Math|Integer|DecrementInt (Variables|/Game/Davidjf5/_Project/Assets/Character/Soldier/Blueprints/BP_FirstPersonCharacterMain.BP_FirstPersonCharacterMain_C|GetMiniboss%20count _character_ref))
      (:%20%20
        (if (<= _result 0)
          (if (<= (Variables|/Game/Davidjf5/_Project/Assets/Character/Soldier/Blueprints/BP_FirstPersonCharacterMain.BP_FirstPersonCharacterMain_C|GetZombie%20Count _character_ref) 0)
            (if (<= (Variables|/Game/Davidjf5/_Project/Assets/Character/Soldier/Blueprints/BP_FirstPersonCharacterMain.BP_FirstPersonCharacterMain_C|GetHellHound%20count _character_ref) 0)
              (Default|BeginRound _character_ref))))))
    (elif (<= (Variables|Default|GetCurrentHealth) 1000)
      (Variables|/Script/Engine.CharacterMovementComponent|SetMaxAcceleration (Variables|Character|GetCharacterMovement) 5e+03))))

(fn ConstructionScript)